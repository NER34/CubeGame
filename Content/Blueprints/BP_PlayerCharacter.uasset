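; Player character for a block-grid world built from chunk actors, with movement, look, jump and a block highlight.
; Enhanced Input stores the move vector and a moving flag; while moving, Tick applies movement and updates the highlight.
; The highlight traces 200 units along the capsule's forward vector, ignoring camera pitch, and snaps Cube to the hit chunk's grid.
; Look input yaws the controller and sets camera rotation through a helper.
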(event Input|EnhancedActionEvents|EnhancedInputActionIA_Move
  (params (ActionValue :type Vector%202D%20Structure) (ElapsedSeconds :type Float%20%28double-precision%29) (TriggeredSeconds :type Float%20%28double-precision%29) (InputAction :type Input%20Action%20Object%20Reference :default "/Game/Inputs/IA_Move.IA_Move"))
  (:Triggered
    (Variables|Default|SetMovementVertor ActionValue))
  (:Started
    (Variables|Default|SetIsMoving true))
  (:Canceled
    (Variables|Default|SetIsMoving false :!label _label))
  (:Completed
    (goto _label)))

(event Input|EnhancedActionEvents|EnhancedInputActionIA_Rotate
  (params (ActionValue :type Vector%202D%20Structure) (ElapsedSeconds :type Float%20%28double-precision%29) (TriggeredSeconds :type Float%20%28double-precision%29) (InputAction :type Input%20Action%20Object%20Reference :default "/Game/Inputs/IA_Rotate.IA_Rotate"))
  (bind (_x _y) (Math|Vector2D|BreakVector2D ActionValue))
  (Pawn|Input|AddControllerYawInput _x)
  (Transformation|SetRelativeRotation (Variables|Default|GetCamera) (|CalcCameraRelativeRotation _y) false false))

(event Input|EnhancedActionEvents|EnhancedInputActionIA_Jump
  (params (ActionValue :type Boolean) (ElapsedSeconds :type Float%20%28double-precision%29) (TriggeredSeconds :type Float%20%28double-precision%29) (InputAction :type Input%20Action%20Object%20Reference :default "/Game/Inputs/IA_Jump.IA_Jump"))
  (:Started
    (Character|Jump)))

(event EventTick
  (params (DeltaSeconds :type Float%20%28single-precision%29))
  (if (Variables|Default|GetIsMoving)
    (CallFunction|UpdatePlayerMovement)
    (CallFunction|HighlightBlock)))

(fn ConstructionScript)

(fn UpdatePlayerMovement
  (bind _movementvertor (Variables|Default|GetMovementVertor))
  (bind (_x _y) (Math|Vector2D|BreakVector2D _movementvertor))
  (Pawn|Input|AddMovementInput (Class|KismetMathLibrary|VectorNormal2D (+ (* (Transformation|GetActorForwardVector) _x) (* _y (Transformation|GetActorRightVector))) 0.0001) 1.0 false))

(fn HighlightBlock
  (bind _capsulecomponent (Variables|Collision|GetCapsuleComponent))
  (bind _returnvalue (Transformation|GetWorldLocation _capsulecomponent))
  (bind _outhit (Collision|LineTraceByChannel _returnvalue (+ _returnvalue (* (Math|Vector|GetForwardVector _capsulecomponent) 2e+02)) "TraceTypeQuery1" false (Utilities|Array|MakeArray self) "None"))
  (bind _aschunk_actor (Utilities|Casting|CastToChunkActor (.HitActor (Collision|BreakHitResult _outhit))))
  (Transformation|SetWorldLocation (Variables|Default|GetCube) (Class|ChunkHelperFunctions|GetBlockRealPos _aschunk_actor (Class|ChunkHelperFunctions|GetBlockGridPos _aschunk_actor (.ImpactPoint (Collision|BreakHitResult _outhit)))) false false))
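; BP_TempChunk is a voxel chunk that renders its blocks as instances of one InstancedStaticMesh.
; Initialize runs the parent setup, then loops over the chunk data and adds a world-space instance for every non-Air block, with no hidden-block culling.
; GetBlockTransform supplies each instance transform, but its MakeTransform from block position and BlockSize is marked unused in the graph.
; BeginPlay, Tick, overlap and construction logic are empty.
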(event EventBeginPlay)

(event Collision|EventActorBeginOverlap
  (params (OtherActor :type Actor%20Object%20Reference)))

(event EventTick
  (params (DeltaSeconds :type Float%20%28single-precision%29)))

(fn ConstructionScript)

(fn Initialize
  (params (InChunkSetup :type Chunk%20Setup%20Structure%20%28by%20ref%29))
  (|CallParentFunction InChunkSetup)
  (for (_array_element _array_index) (Class|ChunkActor|GetChunkData)
    (|BlockIsNotAir _array_element
      (:true
        (Components|InstancedStaticMesh|AddInstance (Variables|Default|GetInstancedStaticMesh) (|GetBlockTransform _array_index) true)))))
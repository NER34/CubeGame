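; BP_ChunkActor is a block-world chunk actor whose Initialize only forwards the chunk setup to its parent class.
; A disconnected loop in Initialize would add an instanced static mesh for each non-air block in the chunk data, filtered by the BlockIsNotAir macro.
; GetBlockTransform holds an unused transform built from block position and size, so this Blueprint itself currently builds no geometry.
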(event EventBeginPlay)

(event Collision|EventActorBeginOverlap
  (params (OtherActor :type Actor%20Object%20Reference)))

(event EventTick
  (params (DeltaSeconds :type Float%20%28single-precision%29)))

(fn ConstructionScript)

(fn Initialize
  (params (InChunkSetup :type Chunk%20Setup%20Structure%20%28by%20ref%29) (InChunkPos :type Int%20Vector%20Structure))
  (|CallParentFunction InChunkSetup ""))
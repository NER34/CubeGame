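; Test pawn that lets the player mine and place blocks in a chunk-based voxel world.
; Each tick a short camera trace is nudged along the hit normal to resolve the mine and place blocks through the chunk generator subsystem.
; Target changes fire an event that resets the timer, moves the highlight and looks up mining time by block type.
; Holding mine advances destruction alpha until the block becomes Air; placing sets Stone.
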(event Input|EnhancedActionEvents|EnhancedInputActionIA_MineCube
  (params (ActionValue :type Boolean) (ElapsedSeconds :type Float%20%28double-precision%29) (TriggeredSeconds :type Float%20%28double-precision%29) (InputAction :type Input%20Action%20Object%20Reference :default "/Game/Inputs/IA_MineCube.IA_MineCube"))
  (:Started
    (Variables|Default|SetbMining true))
  (:Canceled
    (Variables|Default|SetbMining false :!label _label)
    (Variables|Default|SetMiningTimer 0.0)
    (bind _minechunkactor (Variables|Default|GetMineChunkActor)
      (:then
        (Class|ChunkActor|SetBlockDestructionAlpha _minechunkactor (Variables|Default|GetMineBlockPos) 0.0))
      (:else)))
  (:Completed
    (goto _label)))

(event Input|EnhancedActionEvents|EnhancedInputActionIA_PlaceCube
  (params (ActionValue :type Boolean) (ElapsedSeconds :type Float%20%28double-precision%29) (TriggeredSeconds :type Float%20%28double-precision%29) (InputAction :type Input%20Action%20Object%20Reference :default "/Game/Inputs/IA_PlaceCube.IA_PlaceCube"))
  (:Started
    (bind _placechunkactor (Variables|Default|GetPlaceChunkActor)
      (:then
        (Class|ChunkActor|SetBlockType _placechunkactor "Stone" (Variables|Default|GetPlaceBlockPos)))
      (:else))))

(event EventBeginPlay
  (EventDispatchers|BindEventtoOnMiningBlockChanged (EventDispatchers|CreateEvent :!event OnMiningBlockChangedEvent)))

(event EventTick
  (params (DeltaSeconds :type Float%20%28single-precision%29))
  (CallFunction|GetHitBlockData)
  (CallFunction|MineHighlightedBlock DeltaSeconds))

(fn ConstructionScript)

(fn GetHitBlockData
  (bind (_start _end) (|GetTraceEndPoints))
  (LocalVariables|SetPrevMineBlockPos (Variables|Default|GetMineBlockPos))
  (LocalVariables|SetPrevMineChunkActor (Variables|Default|GetMineChunkActor))
  (bind (_outhit _returnvalue) (Collision|LineTraceByChannel _start _end "TraceTypeQuery1" false (Utilities|Array|MakeArray self) "None"))
  (if _returnvalue
    (CallFunction|CollectChunkandBlockPos (Variables|Default|GetPlaceChunkActor) (Variables|Default|GetPlaceBlockPos) (+ (.ImpactPoint (Collision|BreakHitResult _outhit)) (.ImpactNormal (Collision|BreakHitResult _outhit))))
    (bind _blockchanged (CallFunction|CollectChunkandBlockPos (Variables|Default|GetMineChunkActor) (Variables|Default|GetMineBlockPos) (- (.ImpactPoint (Collision|BreakHitResult _outhit)) (.ImpactNormal (Collision|BreakHitResult _outhit)))))
    (if _blockchanged
      (Default|CallOnMiningBlockChanged (Variables|Default|GetMineBlockPos) (Variables|Default|GetMineChunkActor) (LocalVariables|GetPrevMineBlockPos) (LocalVariables|GetPrevMineChunkActor)))
    (else
      (Variables|Default|SetMineChunkActor 0)
      (Variables|Default|SetPlaceChunkActor 0)
      (LocalVariables|GetPrevMineChunkActor
        (:then
          (Default|CallOnMiningBlockChanged :PrevBlockPos (LocalVariables|GetPrevMineBlockPos) :PrevChunkActor (LocalVariables|GetPrevMineChunkActor)))
        (:else)))))

(fn CollectChunkandBlockPos
  (params (ChunkActorRef :type Chunk%20Actor%20Object%20Reference%20%28by%20ref%29) (BlockPosRef :type Int%20Vector%20Structure%20%28by%20ref%29) (PointInWorld :type Vector))
  (bind _returnvalue (Class|ChunkGeneratorSubsystem|GetChunkActor (Subsystems|GetChunkGeneratorSubsystem) (|GetChunkPos)))
  (LocalVariables|SetChunkActor_Local _returnvalue)
  (bind _output_get (LocalVariables|SetChunkChanged_Local (!= (LocalVariables|GetChunkActor_Local) ChunkActorRef)))
  (LocalVariables|SetBlockChangedLocal _output_get)
  (|SetBy-RefVar ChunkActorRef (LocalVariables|GetChunkActor_Local))
  (Utilities|IsValid ChunkActorRef
    (:Is%20Valid
      (LocalVariables|SetBlockPosition_Local (Class|ChunkHelperFunctions|GetBlockGridPos ChunkActorRef PointInWorld))
      (LocalVariables|SetBlockChangedLocal (not (Utilities|Operators|Equal(==) (LocalVariables|GetBlockPosition_Local) BlockPosRef)))
      (|SetBy-RefVar BlockPosRef (LocalVariables|GetBlockPosition_Local)))
    (:Is%20Not%20Valid
      _))
  (return (LocalVariables|GetChunkChanged_Local) (LocalVariables|GetBlockChangedLocal)))

(fn OnMiningBlockChangedEvent
  (params (CurrBlockPos :type Int%20Vector%20Structure) (CurrChunkActor :type Chunk%20Actor%20Object%20Reference) (PrevBlockPos :type Int%20Vector%20Structure) (PrevChunkActor :type Chunk%20Actor%20Object%20Reference))
  (Variables|Default|SetMiningTimer 0.0)
  (Utilities|FlowControl|Sequence
    (:then_0
      (bind _prevchunkactor (LocalVariables|GetPrevChunkActor)
        (:then
          (Class|ChunkActor|SetBlockDestructionAlpha _prevchunkactor PrevBlockPos 0.0)
          (Class|ChunkActor|SetBlockHighlightFlag PrevChunkActor PrevBlockPos false))
        (:else)))
    (:then_1
      (LocalVariables|GetCurrChunkActor
        (:then
          (|ChangeMiningTimeout)
          (Class|ChunkActor|SetBlockHighlightFlag CurrChunkActor CurrBlockPos true))
        (:else)))))

(fn MineHighlightedBlock
  (params (Delta :type Float%20%28double-precision%29))
  (if (Variables|Default|GetbMining)
    (Variables|Default|GetMineChunkActor
      (:then
        (Variables|Default|SetMiningTimer (+ Delta (Variables|Default|GetMiningTimer)))
        (if (>= (Variables|Default|GetMiningTimer) (Variables|Default|GetMiningTimeout))
          (Variables|Default|SetMiningTimer 0.0)
          (Class|ChunkActor|SetBlockType (Variables|Default|GetMineChunkActor) "Air" (Variables|Default|GetMineBlockPos))
          (else
            (Class|ChunkActor|SetBlockDestructionAlpha (Variables|Default|GetMineChunkActor) (Variables|Default|GetMineBlockPos) (/ (Variables|Default|GetMiningTimer) (Variables|Default|GetMiningTimeout))))))
      (:else))))